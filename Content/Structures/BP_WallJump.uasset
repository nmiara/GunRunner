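; BP_WallJump is a toggleable cube structure, named as a wall-jump surface, that can appear and disappear.
; On BeginPlay, IsActive sets the starting visibility of the Cube and the actor's collision.
; Each PlatformActivate event flips both together, reading the Cube's current visibility as the state rather than updating IsActive.
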(event `self.ReceiveBeginPlay`
  (bind _isactive (`self.IsActive`))
  (`SceneComponent.SetVisibility` (`self.Cube`) _isactive false)
  (`self.SetActorEnableCollision` _isactive))

(event `/Game/GunRunner/Interfaces/BPI_PlatformActive.PlatformActivate`
  (if (`SceneComponent.bVisible` (`self.Cube`))
    (`SceneComponent.SetVisibility` (`self.Cube`) false false)
    (`self.SetActorEnableCollision` false)
    (else
      (`SceneComponent.SetVisibility` (`self.Cube`) true false)
      (`self.SetActorEnableCollision` true))))

(fn `UserConstructionScript`)