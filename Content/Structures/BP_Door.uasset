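; BP_Door is a sliding door Blueprint that moves its mesh by a set offset.
; BeginPlay stores the mesh's relative location as the closed position.
; The Open event plays the SlideDoor timeline only when IsOpen is already true, lerping the mesh from closed to offset position without sweep.
; The graph never sets IsOpen and has no closing logic.
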(event `self.ReceiveBeginPlay`
  (set `self.ClosedLocation` (`SceneComponent.RelativeLocation` (`self.DoorMesh`))))

(event `Open`
  (if (`self.bIsOpen`)
    (bind (_direction _alpha) (`Timeline|SlideDoor`)
      (:`Update`
        (`SceneComponent.K2_SetRelativeLocation` (`self.DoorMesh`) (`KismetMathLibrary.VLerp` (`self.ClosedLocation`) (+ (`self.ClosedLocation`) (`self.SlideOffset`)) _alpha) false false)))))

(fn `UserConstructionScript`)