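; BP_CylinderSpikes is a spike cylinder structure that toggles between raised and buried states through PlatformActivate.
; BeginPlay derives the hidden location from the placed one minus BuryDepth, then applies position, visibility and collision from IsActive.
; Each toggle plays or reverses the PlatformRise timeline, which lerps the cylinder between the two locations.
; Visibility and collision switch on before rising and off when the timeline finishes while inactive.
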(event `self.ReceiveBeginPlay`
  (bind _isactive (`self.IsActive`))
  (`SceneComponent.SetVisibility` (`self.SpikeCylinder`) _isactive false)
  (`self.SetActorEnableCollision` _isactive)
  (bind _output_get (set `self.Shown Location` (`SceneComponent.RelativeLocation` (`self.SpikeCylinder`))))
  (set `self.Hidden Location` (- _output_get (`KismetMathLibrary.MakeVector` 0.0 0.0 (`self.Bury Depth`))))
  (if (`self.IsActive`)
    (`SceneComponent.K2_SetRelativeLocation` (`self.SpikeCylinder`) (`self.Shown Location`) false false)
    (`TimelineComponent.SetNewTime` (`self.PlatformRise`) 0.0)
    (else
      (`SceneComponent.K2_SetRelativeLocation` (`self.SpikeCylinder`) (`self.Hidden Location`) false false))))

(event `/Game/GunRunner/Interfaces/BPI_PlatformActive.PlatformActivate`
  (bind _output_get (set `self.IsActive` (!= (`self.IsActive`) true)))
  (if _output_get
    (`SceneComponent.SetVisibility` (`self.SpikeCylinder`) true false)
    (`self.SetActorEnableCollision` true)
    (bind (_direction _newtrack_0) (`Timeline|PlatformRise` :!label _label)
      (:`Update`
        (`SceneComponent.K2_SetRelativeLocation` (`self.SpikeCylinder`) (`KismetMathLibrary.VLerp` (`self.Hidden Location`) (`self.Shown Location`) _newtrack_0) false false))
      (:`Finished`
        (if (not (`self.IsActive`))
          (`SceneComponent.SetVisibility` (`self.SpikeCylinder`) false false)
          (`self.SetActorEnableCollision` false))))
    (else
      (goto _label :!via `Reverse`))))

(fn `UserConstructionScript`)