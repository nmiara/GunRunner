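; BP_ExitDoor is an exit door for Level 1 that opens when the game mode signals an unlock.
; On BeginPlay it casts the game mode to GM_GameModeLevel1 and binds to its DoorUnlock dispatcher.
; On unlock, the OpenDoor timeline slides Cube1 by lerping its world location between the Center and Open components' positions, without sweep.
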(event `self.ReceiveBeginPlay`
  (bind _asgm_game_mode_level_1 (cast `/Game/GameModes/GM_GameModeLevel1` (`GameplayStatics.GetGameMode`)))
  (add `/Game/GameModes/GM_GameModeLevel1.DoorUnlock` _asgm_game_mode_level_1 (delegate `On Door Unlock`)))

(event `On Door Unlock`
  (bind (_direction _newtrack_0) (`Timeline|OpenDoor`)
    (:`Update`
      (`SceneComponent.K2_SetWorldLocation` (`self.Cube1`) (`KismetMathLibrary.VLerp` (`SceneComponent.K2_GetComponentLocation` (`self.Center`)) (`SceneComponent.K2_GetComponentLocation` (`self.Open`)) _newtrack_0) false false))))

(fn `UserConstructionScript`)