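; BP_ActivatablePlatforms is a platform that toggles between shown and buried when PlatformActivate is called.
; BeginPlay derives the hidden location from BuryDepth below the placed cube, then sets position, visibility and collision from IsActive.
; PlatformActivate flips IsActive and plays or reverses the PlatformRise timeline, lerping the cube between both locations.
; Visibility and collision turn on before rising and off only after sinking finishes.
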(event `self.ReceiveBeginPlay`
  (if (`self.IsActive`)
    (`SceneComponent.SetVisibility` (`self.Cube`) true false)
    (`self.SetActorEnableCollision` true)
    (bind _output_get (set `self.ShownLocation` (`SceneComponent.RelativeLocation` (`self.Cube`))))
    (set `self.HiddenLocation` (- _output_get (`KismetMathLibrary.MakeVector` 0.0 0.0 (`self.BuryDepth`))))
    (if (`self.IsActive`)
      (`SceneComponent.K2_SetRelativeLocation` (`self.Cube`) (`self.ShownLocation`) false false)
      (else
        (`SceneComponent.K2_SetRelativeLocation` (`self.Cube`) (`self.HiddenLocation`) false false)))
    (else
      (`SceneComponent.SetVisibility` (`self.Cube`) false false)
      (`self.SetActorEnableCollision` false)
      (bind _output_get_2 (set `self.ShownLocation` (`SceneComponent.RelativeLocation` (`self.Cube`))))
      (set `self.HiddenLocation` (- _output_get_2 (`KismetMathLibrary.MakeVector` 0.0 0.0 (`self.BuryDepth`))))
      (if (`self.IsActive`)
        (`SceneComponent.K2_SetRelativeLocation` (`self.Cube`) (`self.ShownLocation`) false false)
        (else
          (`SceneComponent.K2_SetRelativeLocation` (`self.Cube`) (`self.HiddenLocation`) false false))))))

(event `/Game/GunRunner/Interfaces/BPI_PlatformActive.PlatformActivate`
  (bind _output_get (set `self.IsActive` (!= (`self.IsActive`) true)))
  (if _output_get
    (`SceneComponent.SetVisibility` (`self.Cube`) true false)
    (`self.SetActorEnableCollision` true)
    (bind (_direction _newtrack_0) (`Timeline|PlatformRise` :!label _label)
      (:`Update`
        (`SceneComponent.K2_SetRelativeLocation` (`self.Cube`) (`KismetMathLibrary.VLerp` (`self.HiddenLocation`) (`self.ShownLocation`) _newtrack_0) false false))
      (:`Finished`
        (if (not (`self.IsActive`))
          (`SceneComponent.SetVisibility` (`self.Cube`) false false)
          (`self.SetActorEnableCollision` false))))
    (else
      (goto _label :!via `Reverse`))))

(fn `UserConstructionScript`)