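; BP_CilinderSpikes is a spiked cylinder hazard that damages the player on contact and can optionally move.
; When CanMove is set, a Movement timeline started at BeginPlay lerps the SpikeCylinder between the world locations of components A and B.
; A Box overlap casts the other actor to BP_ShooterCharacter, prints a debug message and calls its AnyDamageEvent.
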(event `self.ReceiveBeginPlay`
  (if (`self.Can Move`)
    (bind (_direction _movement) (`Timeline|Movement` :`NewTime` 5.0)
      (:`Update`
        (`SceneComponent.K2_SetWorldLocation` (`self.SpikeCylinder`) (`KismetMathLibrary.VLerp` (`SceneComponent.K2_GetComponentLocation` (`self.A`)) (`SceneComponent.K2_GetComponentLocation` (`self.B`)) _movement) false false)))))

(event `self.Box.OnComponentBeginOverlap`
  (params (OverlappedComponent :type "PrimitiveComponent Object Reference") (OtherActor :type "Actor Object Reference") (OtherComp :type "PrimitiveComponent Object Reference") (OtherBodyIndex :type Integer) (bFromSweep :type Boolean) (SweepResult :type "HitResult Structure (by ref)"))
  (bind _asbp_shooter_character (cast `/Game/GunRunner/BP_ShooterCharacter` OtherActor))
  (`KismetSystemLibrary.PrintString` "Chocaste con los pinchos")
  (`/Game/GunRunner/BP_ShooterCharacter.AnyDamage_Event` _asbp_shooter_character))

(fn `UserConstructionScript`)