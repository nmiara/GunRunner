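; BP_InteractableColorButton is an unfinished color button structure, set up to receive bullet hits that carry a color.
; SetObjectColor maps a color enum to a blue, red or green material on the Cube's first slot, with green as the fallback.
; OnHitByBullet checks the bullet color but takes no action, and the only SetObjectColor call in the graph is disconnected.
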(event `self.ReceiveBeginPlay`)

(event `OnHitByBullet`
  (params (BulletColor :type "/Game/GunRunner/Blueprints/E_ColorType Enum" :default "NewEnumerator0"))
  (if (`|EnumEquality` BulletColor "NewEnumerator0")
    _))

(event `SetObjectColor`
  (params (ObejctColor :type "/Game/GunRunner/Blueprints/E_ColorType Enum" :default "NewEnumerator0"))
  (if (`|EnumEquality` ObejctColor "NewEnumerator0")
    (`PrimitiveComponent.SetMaterial` (`self.Cube`) 0 "/Game/Materials/M_Blue.M_Blue")
    (elif (`|EnumEquality` ObejctColor "NewEnumerator1")
      (`PrimitiveComponent.SetMaterial` (`self.Cube`) 0 "/Game/Materials/M_Red.M_Red")
      (else
        (`PrimitiveComponent.SetMaterial` (`self.Cube`) 0 "/Game/Materials/M_Green.M_Green")))))

(fn `UserConstructionScript`)