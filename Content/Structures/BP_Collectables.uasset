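; BP_Collectables is a pickup that bobs in place and awards score when collected.
; On BeginPlay the Movement timeline lerps the Recolectable component between the world positions of the Top and Bottom components.
; An overlap on Recolectable casts the game mode to GM_Base, adds Value to the score and destroys the actor.
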(event `self.ReceiveBeginPlay`
  (bind (_direction _newtrack_0) (`Timeline|Movement`)
    (:`Update`
      (`SceneComponent.K2_SetWorldLocation` (`self.Recolectable`) (`KismetMathLibrary.VLerp` (`SceneComponent.K2_GetComponentLocation` (`self.Top`)) (`SceneComponent.K2_GetComponentLocation` (`self.Bottom`)) _newtrack_0) false false))))

(event `self.Recolectable.OnComponentBeginOverlap`
  (params (OverlappedComponent :type "PrimitiveComponent Object Reference") (OtherActor :type "Actor Object Reference") (OtherComp :type "PrimitiveComponent Object Reference") (OtherBodyIndex :type Integer) (bFromSweep :type Boolean) (SweepResult :type "HitResult Structure (by ref)"))
  (bind _asgm_base (cast `/Game/GameModes/GM_Base` (`GameplayStatics.GetGameMode`)))
  (`/Game/GameModes/GM_Base.AddScore` _asgm_base (`self.Value`))
  (`self.K2_DestroyActor`))

(fn `UserConstructionScript`)