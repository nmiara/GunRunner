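; GM_Base is a game mode that tracks elapsed time and coins and handles level victory.
; BeginPlay creates the HUD, Tick accumulates the timer exposed by ReturnTime, and AddCoins pushes the new total to the HUD.
; TriggerVictory, when given a win, plays a sound, disables input, shows WinScreen with the next level name, switches to UI-only input and pauses.
; AddScore is an empty stub.
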(event `self.ReceiveBeginPlay`
  (bind _returnvalue (`|CreateWidget` "/Game/HUD/UMG_HUD.UMG_HUD_C"))
  (bind _output_get (set `self.HUDRef` _returnvalue))
  (`UserWidget.AddToViewport` _output_get 0)
  (set `self.HUDComponent` null))

(event `self.ReceiveTick`
  (params (DeltaSeconds :type "Float (single-precision)"))
  (set `self.Timer` (+ DeltaSeconds (`self.Timer`))))

(event `/Game/GunRunner/Interfaces/BPI_Coin.AddCoins`
  (params (Amount :type Integer))
  (bind _hudref (`self.HUDRef`))
  (set `self.Coins` (+ Amount (`self.Coins`)))
  (`/Engine/EditorBlueprintResources/StandardMacros.IsValid` _hudref
    (:`Is Valid`
      (`/Game/HUD/UMG_HUD.UpdateCoins` _hudref (`self.Coins`)))))

(fn `AddScore`
  (params (Value :type Integer)))

(fn `ReturnTime`
  (returns (time :type "Float (double-precision)"))
  (return (`self.Timer`)))

(fn `TriggerVictory`
  (params (NextLevelName :type Name) (HasWin :type Boolean))
  (bind _output_get (set `self.HasWin` HasWin))
  (if _output_get
    (`GameplayStatics.PlaySound2D` "/Game/Audio/SW_Win.SW_Win" 1.0 1.0 0.0 null null)
    (`self.DisableInput` (`GameplayStatics.GetPlayerController` 0))
    (set `self.HasWin` false)
    (bind _returnvalue (`|CreateWidget` "/Game/HUD/MenusInterface/WinScreen.WinScreen_C" null NextLevelName))
    (`UserWidget.AddToViewport` _returnvalue 0)
    (set `PlayerController.bShowMouseCursor` true (`GameplayStatics.GetPlayerController` 0))
    (`WidgetBlueprintLibrary.SetInputMode_UIOnlyEx` (`GameplayStatics.GetPlayerController` 0) null)
    (`GameplayStatics.SetGamePaused` true)))

(fn `UserConstructionScript`)