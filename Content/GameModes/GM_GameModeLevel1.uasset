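; Game mode for Level 1 that tracks the player's score and unlocks a door once the winning score is reached.
; On BeginPlay it creates the HUD widget, adds it to the viewport and stores it for later updates.
; AddScore increases the score, refreshes the HUD and runs CheckScore, which calls DoorUnlock at or above ScoreToWin.
; A separate OpenLevel function loads the next level by name.
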(event `self.ReceiveBeginPlay`
  (bind _returnvalue (`|GenericCreateObject` (`GameplayStatics.GetPlayerPawn` 0) "/Game/HUD/UMG_HUD.UMG_HUD_C"))
  (`UserWidget.AddToViewport` _returnvalue 0)
  (set `self.HUDComponent` _returnvalue))

(fn `AddScore`
  (params (Value :type Integer))
  (bind _output_get (set `self.Score` (+ Value (`self.Score`))))
  (`/Game/HUD/UMG_HUD.UpdateScore` (`self.HUDComponent`) _output_get)
  (`self.CheckScore`))

(fn `CheckScore`
  (if (>= (`self.Score`) (`self.ScoreToWin`))
    (`self.DoorUnlock`)))

(fn `OpenLevel`
  (params (NextLevel :type String))
  (`GameplayStatics.OpenLevel` (`KismetStringLibrary.Conv_StringToName` NextLevel)))

(fn `UserConstructionScript`)