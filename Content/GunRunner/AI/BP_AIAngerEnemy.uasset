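; Color-matched AI enemy that becomes enraged when shot with the wrong bullet color.
; A matching bullet passes to the parent hit handler unless the enemy is invulnerable.
; A mismatch starts a three-second rage with invulnerability, faster movement, a sound and an angry material.
; When rage ends, it restores normal speed and the original materials cached at BeginPlay.
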(event `self.ReceiveBeginPlay`
  (`parent.ReceiveBeginPlay`)
  (set `self.OriginalMat0` (`PrimitiveComponent.GetMaterial` (`self.Mesh`) 0))
  (set `self.OriginalMat1` (`PrimitiveComponent.GetMaterial` (`self.Mesh`) 1)))

(event `/Game/GunRunner/Interfaces/BPI_Interactable.OnHitByBullet`
  (params (BulletColor :type "/Game/GunRunner/Blueprints/E_ColorType Enum" :default "NewEnumerator0"))
  ; Checa si la bala es del color del enemigo, si no, lo enoja por unos segundos y le saca el enojo, mientras esta enojado es inmortal y corre mas rapido, si impacta la bala correcta y no es invulnerable llama a la funcion del padre y lo elimina
  (if (`|EnumEquality` BulletColor (`self.EnemyColor`))
    (if (not (`self.bIsInvulnerable`))
      (`parent.OnHitByBullet` BulletColor))
    (elif (not (`self.bIsEnraged`))
      (`self.EnterEnragedState`)
      (`KismetSystemLibrary.Delay` 3.0)
      (`self.ResetEnrage`))))

(event `EnterEnragedState`
  ; Entra al estado de furia en el que es inmune y aumenta su velocidad
  (`GameplayStatics.SpawnSoundAttached` "/Game/Audio/SW_Enraged.SW_Enraged" (`self.Mesh`) "None" (0.0 0.0 0.0) (struct) "KeepRelativeOffset" false 1.0 1.0 0.0 "/Game/Audio/SA_Enraged.SA_Enraged" null)
  (set `self.bIsEnraged` true)
  (set `self.bIsInvulnerable` true)
  (set `CharacterMovementComponent.MaxWalkSpeed` (`self.EnragedSpeed`) (`self.CharacterMovement`))
  (`PrimitiveComponent.SetMaterial` (`self.Mesh`) 0 "/Game/Materials/EnemyMaterials/M_AngryState.M_AngryState")
  (`PrimitiveComponent.SetMaterial` (`self.Mesh`) 1 "/Game/Materials/EnemyMaterials/M_AngryState.M_AngryState"))

(event `ResetEnrage`
  ; Reseteo de variables
  (set `self.bIsEnraged` false)
  (set `self.bIsInvulnerable` false)
  (set `CharacterMovementComponent.MaxWalkSpeed` (`self.NormalSpeed`) (`self.CharacterMovement`))
  (`PrimitiveComponent.SetMaterial` (`self.Mesh`) 0 (`self.OriginalMat0`))
  (`PrimitiveComponent.SetMaterial` (`self.Mesh`) 1 (`self.OriginalMat1`)))

(fn `UserConstructionScript`
  (`parent.UserConstructionScript`))