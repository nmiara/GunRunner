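; Shielded AI enemy that blocks bullets until hit by one matching its shield color.
; On BeginPlay it creates a dynamic shield material and tints it blue, red or green from ShieldColor.
; A matching bullet destroys the shield mesh, while others only play a bounce sound.
; Once the shield is gone, bullet hits pass to the parent enemy's handling.
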(event `self.ReceiveBeginPlay`
  (`parent.ReceiveBeginPlay`)
  (bind _returnvalue (`PrimitiveComponent.CreateDynamicMaterialInstance` (`self.ShieldMesh`) 0 "/Game/Materials/M_Shield.M_Shield" "None"))
  (`MaterialInstanceDynamic.SetVectorParameterValue` _returnvalue "Shield" (select `/Game/GunRunner/Blueprints/E_ColorType` (`self.ShieldColor`) :`NewEnumerator0` (struct :`R` 0.045186 :`B` 1.0 :`A` 1.0) :`NewEnumerator1` (struct :`R` 1.0 :`G` 0.020289 :`A` 1.0) :`NewEnumerator2` (struct :`R` 0.051269 :`G` 1.0 :`B` 0.242281 :`A` 1.0) :!type "LinearColor Structure")))

(event `/Game/GunRunner/Interfaces/BPI_Interactable.OnHitByBullet`
  (params (BulletColor :type "/Game/GunRunner/Blueprints/E_ColorType Enum" :default "NewEnumerator0"))
  (if (`self.HasShield`)
    (if (`|EnumEquality` BulletColor (`self.ShieldColor`))
      (set `self.HasShield` false)
      (`ActorComponent.K2_DestroyComponent` (`self.ShieldMesh`))
      (else
        (`GameplayStatics.PlaySound2D` "/Game/Audio/SW_Bounce.SW_Bounce" 1.0 1.0 0.0 null null)))
    (else
      (`parent.OnHitByBullet` BulletColor))))

(fn `UserConstructionScript`
  (`parent.UserConstructionScript`))