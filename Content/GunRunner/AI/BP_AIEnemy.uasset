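; Color-coded AI enemy for GunRunner that is destroyed only by a bullet matching its color.
; BeginPlay applies a blue, red or green material from EnemyColor.
; AI Perception updates write the sensing result to the "HasSeenPlayer?" Blackboard key, while Tick draws a debug view cone from the eyes.
; Box overlap with BP_ShooterCharacter prints a game-over message and calls the player's AnyDamageEvent.
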(event `self.ReceiveTick`
  (params (DeltaSeconds :type "Float (single-precision)"))
  (bind (_outlocation _outrotation) (`self.GetActorEyesViewPoint`))
  (`KismetSystemLibrary.DrawDebugConeInDegrees` _outlocation (`KismetMathLibrary.Conv_RotatorToVector` _outrotation) 2000.0 45.0 45.0 12 (struct :`R` 0.031129 :`B` 1.0 :`A` 1.0)))

(event `self.AIPerception.OnTargetPerceptionUpdated`
  (params (Actor :type "Actor Object Reference") (Stimulus :type "AIStimulus Structure"))
  (bind _returnvalue (`AIBlueprintHelperLibrary.GetBlackboard` (`AIBlueprintHelperLibrary.GetAIController` self)))
  (if Stimulus_bSuccessfullySensed
    (`BlackboardComponent.SetValueAsBool` _returnvalue "HasSeenPlayer?" true)
    (else
      (`BlackboardComponent.SetValueAsBool` _returnvalue "HasSeenPlayer?" false))))

(event `self.ReceiveBeginPlay`
  (`/Game/GunRunner/Interfaces/BPI_Interactable.SetObjectColor` (`self.EnemyColor`)))

(event `/Game/GunRunner/Interfaces/BPI_Interactable.OnHitByBullet`
  (params (BulletColor :type "/Game/GunRunner/Blueprints/E_ColorType Enum" :default "NewEnumerator0"))
  (if (`|EnumEquality` BulletColor (`self.EnemyColor`))
    (`self.K2_DestroyActor`)))

(event `/Game/GunRunner/Interfaces/BPI_Interactable.SetObjectColor`
  (params (ObejctColor :type "/Game/GunRunner/Blueprints/E_ColorType Enum" :default "NewEnumerator0"))
  (if (`|EnumEquality` ObejctColor "NewEnumerator0")
    (`PrimitiveComponent.SetMaterial` (`self.Mesh`) 0 "/Game/Materials/M_Blue.M_Blue")
    (elif (`|EnumEquality` ObejctColor "NewEnumerator1")
      (`PrimitiveComponent.SetMaterial` (`self.Mesh`) 0 "/Game/Materials/M_Red.M_Red")
      (else
        (`PrimitiveComponent.SetMaterial` (`self.Mesh`) 0 "/Game/Materials/M_Green.M_Green")))))

(event `self.Box.OnComponentBeginOverlap`
  (params (OverlappedComponent :type "PrimitiveComponent Object Reference") (OtherActor :type "Actor Object Reference") (OtherComp :type "PrimitiveComponent Object Reference") (OtherBodyIndex :type Integer) (bFromSweep :type Boolean) (SweepResult :type "HitResult Structure (by ref)"))
  (bind _asbp_shooter_character (cast `/Game/GunRunner/BP_ShooterCharacter` OtherActor))
  (`KismetSystemLibrary.PrintString` "Choque con el jugador GameOver")
  (`/Game/GunRunner/BP_ShooterCharacter.AnyDamage_Event` _asbp_shooter_character))

(fn `UserConstructionScript`)