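; A falling platform for GunRunner that sinks when the player pawn overlaps its Box trigger.
; BeginPlay stores the Cube's starting relative location and a hidden location BuryDepth below it.
; The overlap plays the PlatformRise timeline, which lerps the Cube from shown to hidden despite its name.
; PlatformActivate is an empty event, and the hide and collision-disable step on finish is switched off by a constant condition.
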(event `self.ReceiveBeginPlay`
  (bind _output_get (set `self.ShownLocation` (`SceneComponent.RelativeLocation` (`self.Cube`))))
  (set `self.HiddenLocation` (- _output_get (`KismetMathLibrary.MakeVector` 0.0 0.0 (`self.BuryDepth`)))))

(event `self.PlatformActivate`)

(event `self.Box.OnComponentBeginOverlap`
  (params (OverlappedComponent :type "PrimitiveComponent Object Reference") (OtherActor :type "Actor Object Reference") (OtherComp :type "PrimitiveComponent Object Reference") (OtherBodyIndex :type Integer) (bFromSweep :type Boolean) (SweepResult :type "HitResult Structure (by ref)"))
  (if (== OtherActor (`GameplayStatics.GetPlayerPawn` 0))
    (bind (_direction _newtrack_0) (`Timeline|PlatformRise`)
      (:`Update`
        (`SceneComponent.K2_SetRelativeLocation` (`self.Cube`) (`KismetMathLibrary.VLerp` (`self.ShownLocation`) (`self.HiddenLocation`) _newtrack_0) false false))
      (:`Finished`
        (if (not true)
          (`SceneComponent.SetVisibility` (`self.Cube`) false false)
          (`self.SetActorEnableCollision` false))))))

(fn `UserConstructionScript`)